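; BP_Enemy is an enemy actor that currently holds itself at the position where it spawned.
; BeginPlay caches that location, and Tick sets the actor back to it every frame without sweeping.
; Disconnected nodes, which never run, would turn it toward player pawn 0 and step it a fixed distance along that direction, without delta-time scaling.
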(event EventBeginPlay
  (Variables|Default|SetInitialLocation (Transformation|GetActorLocation)))

(event Collision|EventActorBeginOverlap
  (params (OtherActor :type Actor%20Object%20Reference)))

(event EventTick
  (params (DeltaSeconds :type Float%20%28single-precision%29))
  (Transformation|SetActorLocation (Variables|Default|GetInitialLocation) false false))

(fn ConstructionScript)